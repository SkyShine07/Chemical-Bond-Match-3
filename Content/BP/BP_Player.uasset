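; Player pawn Blueprint that handles basic movement through Enhanced Input.
; On BeginPlay it adds the IMC_Default mapping context to player controller 0's input subsystem.
; IMA_Move's 2D value feeds AddMovementInput, with Y along the forward vector and X along the right vector.
; Both directions come from the player controller actor rather than the pawn itself.
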(event Input|EnhancedActionEvents|EnhancedInputActionIA_Move
  (params (ActionValue :type Vector%202D%20Structure) (ElapsedSeconds :type Float%20%28double-precision%29) (TriggeredSeconds :type Float%20%28double-precision%29) (InputAction :type Input%20Action%20Object%20Reference :default "/Game/BP/Input/IA_Move.IA_Move"))
  (bind (_x _y) (Math|Vector2D|BreakVector2D ActionValue))
  (bind _returnvalue (Game|GetPlayerController 0))
  (Pawn|Input|AddMovementInput (* _y (Transformation|GetActorForwardVector _returnvalue)) 1.0 false)
  (Pawn|Input|AddMovementInput (* _x (Transformation|GetActorRightVector _returnvalue)) 1.0 false))

(event EventBeginPlay
  (Input|AddMappingContext (PlayerController|LocalPlayerSubsystems|GetEnhancedInputLocalPlayerSubsystem (Game|GetPlayerController 0)) "/Game/BP/Input/IMC_Default.IMC_Default" 0 "(bIgnoreAllPressedKeysUntilRelease=True,bForceImmediately=False,bNotifyUserSettings=False)"))

(fn ConstructionScript)