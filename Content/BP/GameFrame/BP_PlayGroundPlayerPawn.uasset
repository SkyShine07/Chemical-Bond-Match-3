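; Playground player pawn that starts the GameDirector's region refresh on BeginPlay and visualizes its spatial regions for debugging.
; It binds to the director's region-refreshed event and prints the current main guide region index on each refresh.
; Pressing 1 draws scaled debug spheres at each atom-life grid region's center, plus boxes for the view, logic and atom-life ranges, all placed relative to the pawn.
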(event Custom|OnRegionRefresh
  (params (MainGuideRegion :type Refresh%20Region%20Info%20Structure))
  (Development|PrintText (Utilities|Text|FormatText "当前住区域刷新：{Index}" (Variables|/Script/ChemicalBond.ChemicalBondGameDirector|GetCurrentMainGuideIndex (Variables|Default|GetGameDirector)))))

(event EventBeginPlay
  (bind _asplayground_game_mode (Utilities|Casting|CastToPlaygroundGameMode (Game|GetGameMode)))
  (bind _output_get (Variables|Default|SetGameDirector (Class|ChemicalBondGameMode|GetGameDirector _asplayground_game_mode)))
  (EventDispatchers|BindEventtoOnRegionRefreshed _output_get (EventDispatchers|CreateEvent :!event Custom|OnRegionRefresh))
  (Class|ChemicalBondGameDirector|StartRefreshRegion (Variables|Default|GetGameDirector)))

(event Input|KeyboardEvents|1
  (params (Key :type Key%20Structure :default "None"))
  (:Pressed
    (CallFunction|DrawAtomLifeBox8 0.1)
    (CallFunction|DrawRangeBox3 0.1)))

(fn ConstructionScript)

(fn DrawAtomLifeBox8
  (params (Scale :type Float%20%28single-precision%29))
  (bind _asplayground_game_mode (Utilities|Casting|CastToPlaygroundGameMode (Game|GetGameMode)))
  (bind _returnvalue (Class|ChemicalBondGameDirector|GetAllGridRegionsInfoatAtomLifeRegion (Class|ChemicalBondGameMode|GetGameDirector _asplayground_game_mode) Scale))
  (bind _array_element (Utilities|Array|ForEachLoopwithBreak _returnvalue)
    (:LoopBody
      (Rendering|Debug|DrawDebugSphere (+ (* (+ (.MinRange (Utilities|Struct|BreakRefreshRegionInfo _array_element)) (.MaxRange (Utilities|Struct|BreakRefreshRegionInfo _array_element))) 0.5) (Transformation|GetActorLocation)) 5e+01 12 "(R=1.000000,G=0.039948,B=0.049497,A=1.000000)" 5.0 5.0))))

(fn DrawRangeBox3
  (params (Scale :type Float%20%28single-precision%29))
  (bind _returnvalue (Transformation|GetActorLocation))
  (bind _asplayground_game_mode (Utilities|Casting|CastToPlaygroundGameMode (Game|GetGameMode)))
  (Rendering|Debug|DrawDebugBox _returnvalue (* (Class|ChemicalBondGameDirector|GetViewBoxRange (Class|ChemicalBondGameMode|GetGameDirector _asplayground_game_mode)) Scale) "(R=0.193234,G=1.000000,B=0.083724,A=1.000000)" "0, 0, 0" 15.0 5.0)
  (Rendering|Debug|DrawDebugBox _returnvalue (* (Class|ChemicalBondGameDirector|GetLogicRegionBoxRange (Class|ChemicalBondGameMode|GetGameDirector _asplayground_game_mode)) Scale) "(R=0.044029,G=0.136200,B=1.000000,A=1.000000)" "0, 0, 0" 15.0 5.0)
  (Rendering|Debug|DrawDebugBox _returnvalue (* (Class|ChemicalBondGameDirector|GetAtomLifeRegionBoxRange (Class|ChemicalBondGameMode|GetGameDirector _asplayground_game_mode)) Scale) "(R=1.000000,G=0.019212,B=0.144682,A=1.000000)" "0, 0, 0" 15.0 5.0))