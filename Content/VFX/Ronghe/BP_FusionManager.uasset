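; BP_FusionManager rebuilds the CRT_Fusion render target every tick as a player-centered, top-down map of nearby atom interaction areas for a fusion VFX.
; It gathers all BP_DummyAtom actors, keeping those with CurrentSlots above zero and within 512 units of the player pawn in XY.
; Each is stamped with M_AtomBrush, sized by InteractionRadius and placed by world offset, one unit per pixel, around a fixed 512-pixel center.
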(event EventBeginPlay)

(event Collision|EventActorBeginOverlap
  (params (OtherActor :type Actor%20Object%20Reference)))

(event EventTick
  (params (DeltaSeconds :type Float%20%28single-precision%29))
  (bind _returnvalue (Game|Player|GetPlayerPawn 0))
  (bind _returnvalue_2 (Transformation|GetActorLocation _returnvalue))
  (Rendering|ClearRenderTarget2D "/Game/VFX/Ronghe/CRT_Fusion.CRT_Fusion")
  (bind (_canvas _size _context) (Rendering|BeginDrawCanvastoRenderTarget "/Game/VFX/Ronghe/CRT_Fusion.CRT_Fusion"))
  (bind _outactors (Actor|GetAllActorsOfClass "/Game/VFX/Ronghe/BP_DummyAtom.BP_DummyAtom_C"))
  (for _array_element _outactors
    (bind _asbp_dummy_atom (Utilities|Casting|CastToBP_DummyAtom _array_element))
    (if (> (Variables|/Game/VFX/Ronghe/BP_DummyAtom.BP_DummyAtom_C|GetCurrentSlots _asbp_dummy_atom) 0)
      (if (< (Math|Vector|VectorLengthXY (- _returnvalue_2 (Transformation|GetActorLocation _array_element))) 512.0)
        (Canvas|DrawMaterial :self _canvas :RenderMaterial "/Game/VFX/Ronghe/M_AtomBrush.M_AtomBrush" :ScreenPosition (- (Math|Vector2D|MakeVector2D (+ (.x (- (Transformation|GetActorLocation _array_element) _returnvalue_2)) 512.0) (+ (.y (- (Transformation|GetActorLocation _array_element) _returnvalue_2)) 512.0)) (Math|Vector2D|MakeVector2D (Variables|/Game/VFX/Ronghe/BP_DummyAtom.BP_DummyAtom_C|GetInteractionRadius _asbp_dummy_atom) (Variables|/Game/VFX/Ronghe/BP_DummyAtom.BP_DummyAtom_C|GetInteractionRadius _asbp_dummy_atom))) :ScreenSize (Math|Vector2D|MakeVector2D (* (Variables|/Game/VFX/Ronghe/BP_DummyAtom.BP_DummyAtom_C|GetInteractionRadius _asbp_dummy_atom) 2.0) (* (Variables|/Game/VFX/Ronghe/BP_DummyAtom.BP_DummyAtom_C|GetInteractionRadius _asbp_dummy_atom) 2.0)) :CoordinateSize "(X=1.000000,Y=1.000000)" :PivotPoint "(X=0.000000,Y=0.000000)"))))
  (Rendering|EndDrawCanvastoRenderTarget _context))

(fn ConstructionScript)