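; BP_DummyAtom is a VFX actor that drifts randomly as a placeholder atom.
; A looping timer started on BeginPlay periodically picks a new target at a fixed distance in a random direction from its current position.
; Tick eases the actor toward that target with VInterpTo, zeroing the target's Z so movement settles onto the world Z=0 plane.
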(event Custom|UpdateTarget
  (Variables|Default|SetTargetLocation (+ (Transformation|GetActorLocation) (* (Math|Random|RandomUnitVector) 2e+02))))

(event EventBeginPlay
  (Utilities|Time|SetTimerbyEvent (delegate Custom|UpdateTarget) 1.5 true))

(event Collision|EventActorBeginOverlap
  (params (OtherActor :type Actor%20Object%20Reference)))

(event EventTick
  (params (DeltaSeconds :type Float%20%28single-precision%29))
  (Transformation|SetActorLocation (Math|Interpolation|VInterpTo (Transformation|GetActorLocation) (+ (* (Variables|Default|GetTargetLocation) "1.000000,1.000000,0.000000") "") DeltaSeconds 0.5) false false))

(fn ConstructionScript)